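; Teleporter actor that signals whether something is inside its Box trigger; no teleport logic is in this Blueprint.
; Box begin overlap sets IsTrigger and turns its meshes Green, while end overlap clears the flag and turns them Red, with no filter on the overlapping actor.
; Hide and Show toggle mesh visibility, with Show acting only when Selected is false; neither is called here.
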(event `self.Box.OnComponentBeginOverlap`
  (params (OverlappedComponent :type "PrimitiveComponent Object Reference") (OtherActor :type "Actor Object Reference") (OtherComp :type "PrimitiveComponent Object Reference") (OtherBodyIndex :type Integer) (bFromSweep :type Boolean) (SweepResult :type "HitResult Structure (by ref)"))
  (`self.setActive`)
  (set `self.isTrigger` true))

(event `self.Box.OnComponentEndOverlap`
  (params (OverlappedComponent :type "PrimitiveComponent Object Reference") (OtherActor :type "Actor Object Reference") (OtherComp :type "PrimitiveComponent Object Reference") (OtherBodyIndex :type Integer))
  (`self.setInactive`)
  (set `self.isTrigger` false))

(fn `Hide`
  (`SceneComponent.SetVisibility` (`self.StaticMesh3`) false false)
  (`SceneComponent.SetVisibility` (`self.Auxi`) false false)
  (`SceneComponent.SetVisibility` (`self.StaticMesh`) false false)
  (`SceneComponent.SetVisibility` (`self.StaticMesh1`) false false)
  (`SceneComponent.SetVisibility` (`self.StaticMesh2`) false false)
  (`SceneComponent.SetVisibility` (`self.Main`) false false)
  (`SceneComponent.SetVisibility` (`self.StaticMesh4`) false false)
  (`SceneComponent.SetVisibility` (`self.StaticMesh5`) false false)
  (`SceneComponent.SetVisibility` (`self.StaticMesh6`) false false)
  (`SceneComponent.SetVisibility` (`self.Cube`) false false))

(fn `setActive`
  (`PrimitiveComponent.SetMaterial` (`self.StaticMesh3`) 0 "/Game/Materials/green.green")
  (`PrimitiveComponent.SetMaterial` (`self.StaticMesh1`) 0 "/Game/Materials/green.green")
  (`PrimitiveComponent.SetMaterial` (`self.Auxi`) 0 "/Game/Materials/green.green")
  (`PrimitiveComponent.SetMaterial` (`self.StaticMesh2`) 0 "/Game/Materials/green.green")
  (`PrimitiveComponent.SetMaterial` (`self.StaticMesh`) 0 "/Game/Materials/green.green")
  (`PrimitiveComponent.SetMaterial` (`self.StaticMesh4`) 0 "/Game/Materials/green.green")
  (`PrimitiveComponent.SetMaterial` (`self.StaticMesh5`) 0 "/Game/Materials/green.green")
  (`PrimitiveComponent.SetMaterial` (`self.StaticMesh6`) 0 "/Game/Materials/green.green")
  (`PrimitiveComponent.SetMaterial` (`self.Cube`) 0 "/Game/Materials/green.green"))

(fn `setInactive`
  (`PrimitiveComponent.SetMaterial` (`self.StaticMesh3`) 0 "/Game/Materials/red.red")
  (`PrimitiveComponent.SetMaterial` (`self.StaticMesh1`) 0 "/Game/Materials/red.red")
  (`PrimitiveComponent.SetMaterial` (`self.Auxi`) 0 "/Game/Materials/red.red")
  (`PrimitiveComponent.SetMaterial` (`self.StaticMesh2`) 0 "/Game/Materials/red.red")
  (`PrimitiveComponent.SetMaterial` (`self.StaticMesh`) 0 "/Game/Materials/red.red")
  (`PrimitiveComponent.SetMaterial` (`self.StaticMesh4`) 0 "/Game/Materials/red.red")
  (`PrimitiveComponent.SetMaterial` (`self.StaticMesh5`) 0 "/Game/Materials/red.red")
  (`PrimitiveComponent.SetMaterial` (`self.StaticMesh6`) 0 "/Game/Materials/red.red")
  (`PrimitiveComponent.SetMaterial` (`self.Cube`) 0 "/Game/Materials/red.red"))

(fn `Show`
  (if (not (`self.selected`))
    (`SceneComponent.SetVisibility` (`self.StaticMesh3`) true false)
    (`SceneComponent.SetVisibility` (`self.Auxi`) true false)
    (`SceneComponent.SetVisibility` (`self.StaticMesh`) true false)
    (`SceneComponent.SetVisibility` (`self.StaticMesh1`) true false)
    (`SceneComponent.SetVisibility` (`self.StaticMesh2`) true false)
    (`SceneComponent.SetVisibility` (`self.Main`) true false)
    (`SceneComponent.SetVisibility` (`self.StaticMesh4`) true false)
    (`SceneComponent.SetVisibility` (`self.StaticMesh5`) true false)
    (`SceneComponent.SetVisibility` (`self.StaticMesh6`) true false)
    (`SceneComponent.SetVisibility` (`self.Cube`) true false)))

(fn `UserConstructionScript`)