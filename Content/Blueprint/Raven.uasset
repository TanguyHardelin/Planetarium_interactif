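; Raven is a Blueprint wrapper around a SocketIO client that links the game to a Raven server.
; Incoming socket events are relayed through NewMessageFromRaven with event name and JSON data, leaving Raven components to handle them.
; RegisterEvent binds each event name only once, tracked in a list, and SendDataToRaven emits messages on the root namespace.
; Connection success and failure are printed on screen.
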(event `self.SocketIOClient.OnEvent`
  (params (Event :type String) (MessageJson :type "SIOJsonValue Object Reference"))
  ;[1 1 1] On réagit aux event venant de Raven. On appel l'event NewMessageFromRaven et on laisse les RavenCompont gérer
  (`self.NewMessageFromRaven` Event MessageJson))

(event `self.SocketIOClient.OnFail`
  (`KismetSystemLibrary.PrintString` "Failed to connect to Raven" true true (struct :`G` 0.66 :`B` 1.0 :`A` 1.0) 2000.0))

(event `self.SocketIOClient.OnConnected`
  (params (SessionId :type String) (bIsReconnection :type Boolean))
  (`KismetSystemLibrary.PrintString` "Connected to Raven" true true (struct :`G` 0.66 :`B` 1.0 :`A` 1.0) 2000.0))

(fn `registerEvent`
  (params (evtName :type String))
  ;[1 1 1] On regarde si on a pas déjà bind l'event
  (if (not (`KismetArrayLibrary.Array_Contains` (`self.all_registred_event`) evtName))
    (`KismetArrayLibrary.Array_Append` (`self.all_registred_event`) (`|MakeArray` evtName))
    ;[1 1 1] Si l'évent est pas bind on le bind pour qu'on puisse réagir au .on()
    (`SocketIOClientComponent.BindEvent` (`self.SocketIOClient`) evtName "/")))

(fn `sendDataToRaven`
  (params (evt :type String) (data :type "SIOJsonValue Object Reference"))
  (`SocketIOClientComponent.Emit` (`self.SocketIOClient`) evt data "/"))

(fn `UserConstructionScript`)