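; Planet gravitation component that appears intended to move its owning actor along an elliptical orbit in the XY plane, with no force simulation.
; Each Tick adds delta time to CurrentAngle, then sets the owner's transform with X and Y from cosine and sine scaled by Min and Max.
; The trig inputs read Max rather than CurrentAngle, and the transform resets Z, rotation and scale to defaults.
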(event `self.ReceiveTick`
  (params (DeltaSeconds :type "Float (single-precision)"))
  (bind _max (`self.max`))
  ;[1 1 1] Compute new angle
  (set `self.currentAngle` (+ DeltaSeconds (`self.currentAngle`)))
  ;[1 1 1] Set Location
  (`Actor.K2_SetActorTransform` (`self.GetOwner` self) (`KismetMathLibrary.MakeTransform` (`KismetMathLibrary.MakeVector` (* (`KismetMathLibrary.Cos` _max) (`self.min`)) (* (`KismetMathLibrary.Sin` _max) (`self.max`)))) false false))