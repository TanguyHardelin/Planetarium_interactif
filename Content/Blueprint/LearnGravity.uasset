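; LearnGravity is a VR-throwable actor that simulates gravity toward a planet center, as its own hand-written physics.
; An overlapping BP_MotionController becomes its hand, which it follows while gripping, deriving speed from frame-to-frame movement.
; Opening the hand after a grab starts Tick integration of an inverse-square pull, moving the actor without sweep.
; Overlapping anything named "Planet" destroys it; disconnected orbit, movement and scale experiments never run.
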(event `self.ReceiveTick`
  (params (DeltaSeconds :type "Float (single-precision)"))
  (bind _returnvalue (`self.K2_GetActorLocation` self))
  (bind _returnvalue_2 (- (`self.K2_GetActorLocation` self) (`self.planetCenter`)))
  (bind _returnvalue_3 (`KismetMathLibrary.VSize` _returnvalue_2))
  (if (`self.runPhysics`)
    (bind _output_get (set `self.acceleration` (/ (* (`KismetMathLibrary.Normal` _returnvalue_2) (* (`self.planetteMass`) (`self.objectMass`) (`self.G`))) (* _returnvalue_3 _returnvalue_3 0.0001))))
    ;[1 1 1] Compute speed
    (bind _output_get_2 (set `self.speed` (+ (* (* _output_get 100.0) DeltaSeconds) (`self.speed`))))
    (`self.K2_SetActorLocation` self (+ (`self.K2_GetActorLocation` self) (* (* _output_get_2 DeltaSeconds) -100.0)) false false)
    (else
      ;[1 1 1] Check if hand open
      (switch `/Game/VirtualRealityBP/Blueprints/GripEnum` (`/Game/VirtualRealityBP/Blueprints/BP_MotionController.GripState` (`self.MotionController`))
        (:`NewEnumerator0`
          ;;[1 1 1] Run Physics simulation
          (if (`self.initialised`)
            (set `self.runPhysics` true)))
        (:`NewEnumerator2`
          ;[1 1 1] Follow VR hand
          (set `self.initialised` true)
          (`self.K2_SetActorLocation` self (`SceneComponent.K2_GetComponentLocation` (`/Game/VirtualRealityBP/Blueprints/BP_MotionController.MotionController` (`self.MotionController`))) false false)
          ;;[1 1 1] Compute speed
          (set `self.speed` (* (- (`self.oldPosition`) _returnvalue) 2.0))
          (set `self.oldPosition` _returnvalue))))))

(event `self.SphereCollision.OnComponentBeginOverlap`
  (params (OverlappedComponent :type "PrimitiveComponent Object Reference") (OtherActor :type "Actor Object Reference") (OtherComp :type "PrimitiveComponent Object Reference") (OtherBodyIndex :type Integer) (bFromSweep :type Boolean) (SweepResult :type "HitResult Structure (by ref)"))
  (bind _returnvalue (`KismetSystemLibrary.GetObjectName` OtherActor))
  ;[1 1 1] Manage Collision
  (if (`KismetStringLibrary.Contains` _returnvalue "Planet")
    (`self.K2_DestroyActor`)
    (else
      ;;[1 1 1] Check MotionController
      (if (`KismetStringLibrary.Contains` _returnvalue "MotionController")
        (if (not (`self.initialised`))
          (bind _asbp_motion_controller (cast `/Game/VirtualRealityBP/Blueprints/BP_MotionController` OtherActor))
          (set `self.MotionController` _asbp_motion_controller)
          (set `self.MotionControllerAttached` true))))))

(fn `UserConstructionScript`)