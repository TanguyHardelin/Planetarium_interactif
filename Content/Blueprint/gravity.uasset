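; Component that moves its owning actor along an elliptical orbit around Center and spins it on yaw, like simulated planetary motion.
; Tick throttles updates by Ratio, advancing the angle and placing the owner via Cos/Sin scaled by Min and Max, keeping Z.
; Optional TraceBall spawning marks the path, reusing the throttle's Compteur as its interval counter.
; RunGravity and RunRotation toggle orbit and spin independently.
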(event `self.ReceiveTick`
  (params (DeltaSeconds :type "Float (single-precision)"))
  (bind _currentangle (`self.currentAngle`))
  (bind _returnvalue (`self.GetOwner` self))
  (if (> (`self.compteur`) (`self.ratio`))
    (set `self.compteur` 0.0)
    (`|ExecutionSequence`
      (:`then_0`
        (if (`self.runGravity`)
          ;[1 1 1] Compute new angle
          (set `self.currentAngle` (+ (* (`self.ratio`) (`self.ratioGravity`)) (`self.currentAngle`)))
          ;[1 1 1] Set Location
          (`Actor.K2_SetActorTransform` (`self.GetOwner` self) (`KismetMathLibrary.MakeTransform` (+ (`self.center`) (`KismetMathLibrary.MakeVector` (* (`KismetMathLibrary.Cos` _currentangle) (`self.min`)) (* (`KismetMathLibrary.Sin` _currentangle) (`self.max`)) (.z (`Actor.K2_GetActorLocation` _returnvalue)))) (`Actor.K2_GetActorRotation` (`self.GetOwner` self)) (`Actor.GetActorScale3D` _returnvalue)) false false)
          (if (`self.displayTrace`)
            (bind _output_get (set `self.compteur` (+ (`self.compteur`) 1.0)))
            (if (> _output_get (`self.intervaleBetweenBall`))
              (set `self.compteur` 0.0)
              (`|SpawnActorFromClass` "/Game/Blueprint/TraceBall.TraceBall_C" (`KismetMathLibrary.Conv_VectorToTransform` (`Actor.K2_GetActorLocation` (`self.GetOwner` self))) "Undefined" "OverrideRootScale" null null)))))
      (:`then_1`
        ;[1 1 1] Rotation
        ;;[1 1 1] Check if run rotation
        (if (`self.runRotation`)
          ;;[1 1 1] setRotation Value
          (bind _output_get_2 (set `self.rotation` (+ (* DeltaSeconds (`self.ratioRotation`)) (`self.rotation`))))
          ;;[1 1 1] Check if rotation > 360
          (if (> _output_get_2 360.0)
            (set `self.rotation` 0.0))
          ;;[1 1 1] Apply rotation
          (`Actor.K2_SetActorRotation` (`self.GetOwner` self) (`KismetMathLibrary.MakeRotator` 0.0 0.0 (`self.rotation`)) false)
          (else
            (set `self.rotation` 0.0)))))
    (else
      (set `self.compteur` (+ (`self.compteur`) DeltaSeconds)))))