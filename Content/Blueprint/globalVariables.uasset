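; Global state actor for what appears to be a star system sim, holding star mass, object mass and planet center.
; On Tick, a star mass change rescales the habitable-zone meshes BadExterior, BadInterior and Good, found by display name, in X/Y by the mass's square root.
; Planet repositioning is unfinished: its loops are empty and the SetActorLocation nodes are unconnected.
; Helpers return the planet center and add object mass only while the total stays positive.
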(event `self.ReceiveTick`
  (params (DeltaSeconds :type "Float (single-precision)"))
  (bind _returnvalue (* (`KismetMathLibrary.Sqrt` (`self.currentStarMass`)) 1.0))
  ;[1 1 1] Update hability zone
  (if (!= (`self.currentStarOld`) (`self.currentStarMass`))
    (set `self.currentStarOld` (`self.currentStarMass`))
    (bind _outactors (`GameplayStatics.GetAllActorsOfClass` "/Script/Engine.StaticMeshActor"))
    (for _array_element _outactors
      (bind _returnvalue_2 (`KismetSystemLibrary.GetDisplayName` _array_element))
      (if (`KismetStringLibrary.EqualEqual_StrStr` _returnvalue_2 "BadExterior")
        (set `self.habilitabilityScale` (10000.0 10000.0 0.01))
        (`SceneComponent.SetWorldScale3D` (`StaticMeshActor.StaticMeshComponent` _array_element) (* (`self.habilitabilityScale`) (`KismetMathLibrary.MakeVector` _returnvalue _returnvalue 1.0)) :!label _label)
        (elif (`KismetStringLibrary.EqualEqual_StrStr` _returnvalue_2 "BadInterior")
          (set `self.habilitabilityScale` (200.0 200.0 0.01))
          (goto _label)
          (elif (`KismetStringLibrary.EqualEqual_StrStr` _returnvalue_2 "Good")
            (set `self.habilitabilityScale` (470.0 470.0 0.01))
            (goto _label)))))
    ;[1 1 1] set planet location
    (bind _outactors_2 (`GameplayStatics.GetAllActorsOfClass` "/Game/Planet_Creator_1/Blueprint/BP_Planet_1.BP_Planet_1_C"))
    (for _array_element_2 _outactors_2
      _)
    (bind _outactors_3 (`GameplayStatics.GetAllActorsOfClass` "/Game/Planet_Creator_2/Blueprints/BP_Planet_2.BP_Planet_2_C"))
    (for _array_element_3 _outactors_3
      _)))

(fn `addMass`
  (params (mass :type "Float (double-precision)"))
  (bind _returnvalue (+ (`self.currentObjMass`) mass))
  (if (> _returnvalue 0.0)
    (set `self.currentObjMass` _returnvalue)))

(fn `recupCurrentCenter`
  (returns (center :type "Vector Structure"))
  (return (`self.currentPlanetCenter`)))

(fn `UserConstructionScript`)