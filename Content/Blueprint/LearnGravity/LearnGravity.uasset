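; LearnGravity is a VR-held object that teaches gravity: the player grabs and throws it around a planet.
; While held, it follows the motion controller, scales with the mass read from GlobalVariables and derives velocity from hand movement.
; On release, Tick manually integrates inverse-square attraction toward the planet center and periodically spawns TraceBall markers along the path.
; Overlapping a planet destroys it; disconnected orbit experiments remain unused.
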(event `self.ReceiveTick`
  (params (DeltaSeconds :type "Float (single-precision)"))
  (bind _returnvalue (`self.K2_GetActorLocation` self))
  (bind _motioncontroller (`/Game/VirtualRealityBP/Blueprints/BP_MotionController.MotionController` (`self.MotionController`)))
  (bind _returnvalue_2 (- (`self.K2_GetActorLocation` self) (`self.planetCenter`)))
  (bind _returnvalue_3 (`KismetMathLibrary.VSize` _returnvalue_2))
  (if (`self.runPhysics`)
    (`|ExecutionSequence`
      (:`then_0`
        (bind _output_get (set `self.acceleration` (/ (* (`KismetMathLibrary.Normal` _returnvalue_2) (* (`self.planetteMass`) (`self.objectMass`) (`self.G`))) (* _returnvalue_3 _returnvalue_3 0.1))))
        ;[1 1 1] Compute speed
        (bind _output_get_2 (set `self.speed` (+ (* (* _output_get 1.0) DeltaSeconds) (`self.speed`))))
        (`self.K2_SetActorLocation` self (+ (`self.K2_GetActorLocation` self) (* (* _output_get_2 DeltaSeconds) -100.0)) false false))
      (:`then_1`
        (bind _output_get_3 (set `self.compteur` (+ (`self.compteur`) 1.0)))
        (if (> _output_get_3 (`self.intervaleBetweenBall`))
          (set `self.compteur` 0.0)
          (`|SpawnActorFromClass` "/Game/Blueprint/TraceBall.TraceBall_C" (`KismetMathLibrary.MakeTransform` (`self.K2_GetActorLocation` self) (struct) (0.1 0.1 0.1)) "Undefined" "OverrideRootScale" null null))))
    (else
      (bind _outactors (`GameplayStatics.GetAllActorsOfClass` "/Game/Blueprint/globalVariables.globalVariables_C"))
      (bind _output (`|GetArrayItem` _outactors))
      (set `self.planetCenter` (`/Game/Blueprint/globalVariables.currentPlanetCenter` _output))
      (set `self.planetteMass` (`/Game/Blueprint/globalVariables.currentPlanetMass` _output))
      (set `self.objectMass` (`/Game/Blueprint/globalVariables.currentObjMass` _output))
      ;[1 1 1] Check if hand open
      (switch `/Game/VirtualRealityBP/Blueprints/GripEnum` (`/Game/VirtualRealityBP/Blueprints/BP_MotionController.GripState` (`self.MotionController`))
        (:`NewEnumerator0`
          ;;[1 1 1] Run Physics simulation
          (if (`self.initialised`)
            (set `self.runPhysics` true)))
        (:`NewEnumerator2`
          ;[1 1 1] Follow VR hand
          (set `self.initialised` true)
          (bind _outactors_2 (`GameplayStatics.GetAllActorsOfClass` "/Game/Blueprint/globalVariables.globalVariables_C"))
          (bind _returnvalue_4 (/ (`/Game/Blueprint/globalVariables.currentObjMass` (`|GetArrayItem` _outactors_2)) 1000.0))
          (`self.K2_SetActorTransform` self (`KismetMathLibrary.MakeTransform` (`SceneComponent.K2_GetComponentLocation` _motioncontroller) (`SceneComponent.RelativeRotation` _motioncontroller) (`KismetMathLibrary.MakeVector` _returnvalue_4 _returnvalue_4 _returnvalue_4)) false false)
          ;;[1 1 1] Compute speed
          (set `self.speed` (* (- (`self.oldPosition`) _returnvalue) 2.0))
          (set `self.oldPosition` _returnvalue))))))

(event `self.SphereCollision.OnComponentBeginOverlap`
  (params (OverlappedComponent :type "PrimitiveComponent Object Reference") (OtherActor :type "Actor Object Reference") (OtherComp :type "PrimitiveComponent Object Reference") (OtherBodyIndex :type Integer) (bFromSweep :type Boolean) (SweepResult :type "HitResult Structure (by ref)"))
  (bind _returnvalue (`KismetSystemLibrary.GetObjectName` OtherActor))
  ;[1 1 1] Manage Collision
  (if (`KismetStringLibrary.Contains` _returnvalue "Planet")
    (`self.K2_DestroyActor`)
    (else
      ;;[1 1 1] Check MotionController
      (if (`KismetStringLibrary.Contains` _returnvalue "MotionController")
        (if (not (`self.initialised`))
          (bind _asbp_motion_controller (cast `/Game/VirtualRealityBP/Blueprints/BP_MotionController` OtherActor))
          (set `self.MotionController` _asbp_motion_controller)
          (set `self.MotionControllerAttached` true))))))

(fn `UserConstructionScript`)