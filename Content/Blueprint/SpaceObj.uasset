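; SpaceObj is a space object actor with a prototype sphere visual.
; On BeginPlay it scales the sphere uniformly from Size, clamped to a minimum, and assigns itself as the Parent of Trace.
; Tick does nothing; disconnected nodes hold circular orbit logic that would advance Cycle by Period and place DefaultSceneRoot1 at Distance in the XY plane, preserving height, rotation and scale.
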(event `self.ReceiveBeginPlay`
  (`SceneComponent.SetRelativeScale3D` (`self.Sphere`) (* (`KismetMathLibrary.MakeVector` 1.0 1.0 1.0) (`KismetMathLibrary.FMax` (* (`self.size`) 0.001) 0.1)))
  (set `/Game/Trace.parent` self (`self.Trace`)))

(event `self.ReceiveTick`
  (params (DeltaSeconds :type "Float (single-precision)")))

(fn `UserConstructionScript`)