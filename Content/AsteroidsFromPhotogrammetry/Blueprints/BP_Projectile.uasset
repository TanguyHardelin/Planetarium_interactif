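; Weapon projectile actor that sets its destructive power from the player's selected weapon and cleans itself up after a hit or a miss.
; The construction script reads CurrentWeapon from BP_FlyingGameInstance to set force, damage radius, mesh scale and color, with Plasma Torpedos as the smaller, weaker variant.
; It also starts a timer that destroys the projectile after a few seconds, while the Hit event destroys it after a brief delay.
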(event `DestroySelf`
  ;[1 1 1] Destroy the projectile actor 2.5 seconds after a miss
  (`/Engine/EditorBlueprintResources/StandardMacros.IsValid` (`self.Projectile`)
    (:`Is Valid`
      (`self.K2_DestroyActor`)
      (`KismetSystemLibrary.K2_ClearTimer` null "DestroySelf"))))

(event `self.ReceiveHit`
  (params (MyComp :type "PrimitiveComponent Object Reference") (Other :type "Actor Object Reference") (OtherComp :type "PrimitiveComponent Object Reference") (bSelfMoved :type Boolean) (HitLocation :type "Vector Structure") (HitNormal :type "Vector Structure") (NormalImpulse :type "Vector Structure") (Hit :type "HitResult Structure (by ref)"))
  ;[1 1 1] Destroy the projectile actor right after a hit
  (`KismetSystemLibrary.Delay` 0.1)
  (`self.K2_DestroyActor`))

(fn `UserConstructionScript`
  (bind _projectile (`self.Projectile`))
  ;[1 1 1] Destroy the projectile actor after 2.5 seconds
  (`KismetSystemLibrary.K2_SetTimer` null "DestroySelf" 2.5)
  ;[1 1 1] Ajdust projectile's destructive power based on the weapon that fired it
  (bind _asbp_flying_game_instance (cast `/Game/AsteroidsFromPhotogrammetry/Blueprints/BP_FlyingGameInstance` (`GameplayStatics.GetGameInstance`))
    (:`then`
      (if (`KismetStringLibrary.EqualEqual_StrStr` (`/Game/AsteroidsFromPhotogrammetry/Blueprints/BP_FlyingGameInstance.Current Weapon` _asbp_flying_game_instance) "Plasma Torpedos")
        (set `self.Force` 125000.0)
        (set `self.Damage Radius` 1000.0)
        (`SceneComponent.SetRelativeScale3D` _projectile (0.5 0.5 0.5))
        (`MeshComponent.SetVectorParameterValueOnMaterials` _projectile "Projectile Color" (0.0 0.176 0.998))
        (else
          (set `self.Force` 300000.0)
          (set `self.Damage Radius` 3000.0)
          (`SceneComponent.SetRelativeScale3D` _projectile (2.0 2.0 2.0))
          (`MeshComponent.SetVectorParameterValueOnMaterials` _projectile "Projectile Color" (0.0 0.15 0.0)))))
    (:`CastFailed`
      (`KismetSystemLibrary.PrintString` "Cast to BP_FlyingGameInstance failed! Please make sure to set the BP_FlyingGameInstance as your project's game instance tin the project's settings."))))