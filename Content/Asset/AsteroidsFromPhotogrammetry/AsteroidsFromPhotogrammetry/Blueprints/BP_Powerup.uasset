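; BP_Powerup is a pickup actor that switches the player's weapon to the Plasma Cannon when the spaceship flies through it.
; On Sphere1 overlap, it identifies the BP_FlyingPawn by display name, plays a sound and destroys itself.
; It then sets the current weapon on BP_FlyingGameInstance and refreshes the HUD, printing a setup warning if the game instance cast fails.
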(event `self.Sphere1.OnComponentBeginOverlap`
  (params (OverlappedComponent :type "PrimitiveComponent Object Reference") (OtherActor :type "Actor Object Reference") (OtherComp :type "PrimitiveComponent Object Reference") (OtherBodyIndex :type Integer) (bFromSweep :type Boolean) (SweepResult :type "HitResult Structure (by ref)"))
  ;[1 1 1] Change the weapon, if the spaceship flies through the spawned Power UP
  (if (`KismetStringLibrary.EqualEqual_StrStr` (`KismetSystemLibrary.GetDisplayName` OtherActor) "BP_FlyingPawn")
    (`GameplayStatics.PlaySound2D` "/Game/AsteroidsFromPhotogrammetry/Sounds/Wavs/A_PowerUp.A_PowerUp")
    (`self.K2_DestroyActor`)
    (bind _asbp_flying_game_instance (cast `/Game/AsteroidsFromPhotogrammetry/Blueprints/BP_FlyingGameInstance` (`GameplayStatics.GetGameInstance`))
      (:`then`
        (set `/Game/AsteroidsFromPhotogrammetry/Blueprints/BP_FlyingGameInstance.Current Weapon` "Plasma Cannon" _asbp_flying_game_instance)
        (`/Game/AsteroidsFromPhotogrammetry/UI/WB_Hud.Update Current Weapon_Event` (`/Game/AsteroidsFromPhotogrammetry/Blueprints/BP_FlyingGameInstance.GameHud` _asbp_flying_game_instance)))
      (:`CastFailed`
        (`KismetSystemLibrary.PrintString` "Cast to BP_FlyingGameInstance failed! Please make sure to set the BP_FlyingGameInstance as your project's game instance tin the project's settings.")))))

(fn `UserConstructionScript`)