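; Star anomaly actor: a colored star sphere with an animated, cloudy disk material and two lens flare billboards.
; The construction script pushes editable disk, star and lens settings into dynamic materials on the cube, sphere and billboards.
; Each tick feeds the projected screen position and brightness to both billboards.
; A camera-to-star object trace steps brightness down when blocked and up when clear, clamped to lens luminosity.
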(event `self.ReceiveTick`
  (params (DeltaSeconds :type "Float (single-precision)"))
  (bind _materialbillboard1 (`self.MaterialBillboard1`))
  (bind _materialbillboard (`self.MaterialBillboard`))
  (bind _lens_luminosity (`self.Lens_Luminosity`))
  (bind _screenposition (`GameplayStatics.ProjectWorldToScreen` (`GameplayStatics.GetPlayerController` 0) (`SceneComponent.K2_GetComponentLocation` (`self.MaterialBillboard`))))
  (bind _returnvalue (`KismetMathLibrary.FClamp` (+ (`self.Brightness`) -0.05) 0.0 _lens_luminosity))
  (bind _returnvalue_2 (`KismetMathLibrary.FClamp` (+ (`self.Brightness`) 0.05) 0.0 _lens_luminosity))
  (bind _returnvalue_3 (`PrimitiveComponent.CreateDynamicMaterialInstance` _materialbillboard1 0 (`PrimitiveComponent.GetMaterial` _materialbillboard1 0)))
  (bind _returnvalue_4 (`PrimitiveComponent.CreateDynamicMaterialInstance` _materialbillboard 0 (`PrimitiveComponent.GetMaterial` _materialbillboard 0)))
  (`MaterialInstanceDynamic.SetScalarParameterValue` _returnvalue_4 "Screen_Position" (/ (`KismetMathLibrary.BreakVector2D` _screenposition) 1000.0))
  (`MaterialInstanceDynamic.SetScalarParameterValue` _returnvalue_3 "Screen_Position" (/ (`KismetMathLibrary.BreakVector2D` _screenposition) 1000.0))
  (`MaterialInstanceDynamic.SetScalarParameterValue` _returnvalue_4 "Screen_Y" (/ (`.Y` (`KismetMathLibrary.BreakVector2D` _screenposition)) 1000.0))
  (`MaterialInstanceDynamic.SetScalarParameterValue` _returnvalue_3 "Screen_Y" (/ (`.Y` (`KismetMathLibrary.BreakVector2D` _screenposition)) 1000.0))
  (`MaterialInstanceDynamic.SetScalarParameterValue` _returnvalue_4 "Brightness" (`self.Brightness`))
  (`MaterialInstanceDynamic.SetScalarParameterValue` _returnvalue_3 "Brightness" (`self.Brightness`))
  (bind (_outhit _returnvalue_5) (`KismetSystemLibrary.LineTraceSingleForObjects` (`SceneComponent.K2_GetComponentLocation` (`PlayerCameraManager.TransformComponent` (`GameplayStatics.GetPlayerCameraManager` 0))) (`SceneComponent.K2_GetComponentLocation` (`self.DefaultSceneRoot`)) (`self.Object_Type`)))
  (if _returnvalue_5
    (set `self.Brightness` _returnvalue)
    (set `self.Size` _returnvalue)
    (else
      (set `self.Brightness` _returnvalue_2)
      (set `self.Size` _returnvalue_2))))

(fn `UserConstructionScript`
  (bind _materialbillboard1 (`self.MaterialBillboard1`))
  (bind _materialbillboard (`self.MaterialBillboard`))
  (bind _sphere (`self.Sphere`))
  (bind _cube (`self.Cube`))
  (bind _returnvalue (`PrimitiveComponent.CreateDynamicMaterialInstance` _cube 0 (`PrimitiveComponent.GetMaterial` _cube 0)))
  (set `self.DMI_Disk` _returnvalue)
  (`|ExecutionSequence`
    (:`then_0`
      (`MaterialInstanceDynamic.SetScalarParameterValue` (`self.DMI_Disk`) "Clouds_Shadows" (`self.Clouds_Shadows`))
      (`MaterialInstanceDynamic.SetScalarParameterValue` (`self.DMI_Disk`) "Core_Disks_Density" (`self.Core_Disks_Density`))
      (`MaterialInstanceDynamic.SetScalarParameterValue` (`self.DMI_Disk`) "Core_Disks_Radius" (`self.Core_Disks_Radius`))
      (`MaterialInstanceDynamic.SetScalarParameterValue` (`self.DMI_Disk`) "Dense_Clouds_Radius" (`self.Dense_Clouds_Radius`))
      (`MaterialInstanceDynamic.SetScalarParameterValue` (`self.DMI_Disk`) "Disk_1_Radius" (`self.Disk_1_Radius`))
      (`MaterialInstanceDynamic.SetScalarParameterValue` (`self.DMI_Disk`) "Disk_2_Radius" (`self.Disk_2_Radius`))
      (`MaterialInstanceDynamic.SetScalarParameterValue` (`self.DMI_Disk`) "Emissive" (`self.Emissive`))
      (`MaterialInstanceDynamic.SetScalarParameterValue` (`self.DMI_Disk`) "Global_Tile" (`self.Global_Tile`))
      (`MaterialInstanceDynamic.SetScalarParameterValue` (`self.DMI_Disk`) "Halo" (`self.Halo`))
      (`MaterialInstanceDynamic.SetScalarParameterValue` (`self.DMI_Disk`) "Inner_Disk_Radius" (`self.Inner_Disk_Radius`))
      (`MaterialInstanceDynamic.SetScalarParameterValue` (`self.DMI_Disk`) "Opacity" (`self.Opacity`))
      (`MaterialInstanceDynamic.SetScalarParameterValue` (`self.DMI_Disk`) "Opacity_Inner_Density" (`self.Opacity_Inner_Density`))
      (`MaterialInstanceDynamic.SetScalarParameterValue` (`self.DMI_Disk`) "Opacity_Inner_Radius" (`self.Opacity_Inner_Radius`))
      (`MaterialInstanceDynamic.SetScalarParameterValue` (`self.DMI_Disk`) "Opacity_Outer_Density" (`self.Opacity_Outer_Density`))
      (`MaterialInstanceDynamic.SetScalarParameterValue` (`self.DMI_Disk`) "Opacity_Outer_Radius" (`self.Opacity_Outer_Radius`))
      (`MaterialInstanceDynamic.SetScalarParameterValue` (`self.DMI_Disk`) "Outer_Disk_Tile_X" (`self.Outer_Disk_Tile_X`))
      (`MaterialInstanceDynamic.SetScalarParameterValue` (`self.DMI_Disk`) "Outer_Disk_Tile_Y" (`self.Outer_Disk_Tile_Y`))
      (`MaterialInstanceDynamic.SetScalarParameterValue` (`self.DMI_Disk`) "Speed" (`self.Speed`))
      (`MaterialInstanceDynamic.SetScalarParameterValue` (`self.DMI_Disk`) "Waves_Speed" (`self.Waves_Speed`))
      (`MaterialInstanceDynamic.SetScalarParameterValue` (`self.DMI_Disk`) "Waves_Strength" (`self.Waves_Strength`)))
    (:`then_1`
      (`MaterialInstanceDynamic.SetVectorParameterValue` (`self.DMI_Disk`) "Disk_1_Color" (`self.Disk_1_Color`))
      (`MaterialInstanceDynamic.SetVectorParameterValue` (`self.DMI_Disk`) "Disk_2_Color" (`self.Disk_2_Color`))
      (`MaterialInstanceDynamic.SetVectorParameterValue` (`self.DMI_Disk`) "Disk_3_Color" (`self.Disk_3_Color`))
      (`MaterialInstanceDynamic.SetVectorParameterValue` (`self.DMI_Disk`) "Halo_Color" (`self.Halo_Color`))
      (`MaterialInstanceDynamic.SetVectorParameterValue` (`self.DMI_Disk`) "Inner_Disk_Color" (`self.Inner_Disk_Color`))
      (`MaterialInstanceDynamic.SetVectorParameterValue` (`self.DMI_Disk`) "Outer_Color" (`self.Outer_Color`)))
    (:`then_2`
      (bind _returnvalue_2 (`PrimitiveComponent.CreateDynamicMaterialInstance` _materialbillboard1 0 (`PrimitiveComponent.GetMaterial` _materialbillboard1 0)))
      (bind _returnvalue_3 (`PrimitiveComponent.CreateDynamicMaterialInstance` _materialbillboard 0 (`PrimitiveComponent.GetMaterial` _materialbillboard 0)))
      (`MaterialInstanceDynamic.SetScalarParameterValue` _returnvalue_3 "Brightness" (`self.Lens_Luminosity`))
      (`MaterialInstanceDynamic.SetScalarParameterValue` _returnvalue_2 "Brightness" (`self.Lens_Luminosity`))
      (`MaterialInstanceDynamic.SetVectorParameterValue` _returnvalue_3 "Color_1" (`self.Lens_Main_Color`))
      (`MaterialInstanceDynamic.SetVectorParameterValue` _returnvalue_2 "Color_1" (`self.Lens_Main_Color`))
      (`MaterialInstanceDynamic.SetVectorParameterValue` _returnvalue_2 "Color_2" (`self.Lens_Outer_Color`))
      (`MaterialInstanceDynamic.SetVectorParameterValue` _returnvalue_3 "Color_2" (`self.Lens_Outer_Color`)))
    (:`then_3`
      (bind _returnvalue_4 (`PrimitiveComponent.CreateDynamicMaterialInstance` _sphere 0 (`PrimitiveComponent.GetMaterial` _sphere 0)))
      (`MaterialInstanceDynamic.SetVectorParameterValue` _returnvalue_4 "Color" (`self.Star_Color`))
      (`MaterialInstanceDynamic.SetScalarParameterValue` _returnvalue_4 "Lumoinosity" (`self.Star_Luminosity`)))))