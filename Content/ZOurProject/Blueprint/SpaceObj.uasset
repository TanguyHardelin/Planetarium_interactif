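; SpaceObj is an actor Blueprint that moves along an elliptical orbit around the world origin in the XY plane.
; Tick adds DeltaSeconds to CurrentAngle, giving a fixed one radian per second, then scales its cosine by MinDistance for X and its sine by MaxDistance for Y.
; The position becomes a whole actor transform without sweep, so rotation and scale reset to defaults each frame.
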(event `self.ReceiveTick`
  (params (DeltaSeconds :type "Float (single-precision)"))
  (bind _current_angle (`self.current_angle`))
  ;[1 1 1] Compute new angle
  (set `self.current_angle` (+ DeltaSeconds (`self.current_angle`)))
  ;[1 1 1] Set Location
  (`self.K2_SetActorTransform` self (`KismetMathLibrary.Conv_VectorToTransform` (`KismetMathLibrary.MakeVector` (* (`KismetMathLibrary.Cos` _current_angle) (`self.min_distance`)) (* (`KismetMathLibrary.Sin` _current_angle) (`self.max_distance`)))) false false))

(fn `UserConstructionScript`)