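; Manager actor that mirrors externally supplied space-simulation data as SpaceObj actors in the level.
; It listens to RavenComponent messages and parses their JSON object arrays.
; "All Space Obj" spawns an actor per entry with position, name and speed, tracking it in AllObjects.
; "New Simulation" matches entries to tracked actors by name through a nested loop and sets their transforms from position alone.
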(event `self.RavenComponent.onRavenMessage`
  (params (eventName :type String) (data :type "SIOJsonValue Object Reference"))
  (switch `string` eventName
    (:`allSpaceObj`
      (bind _returnvalue (`SIOJsonValue.AsObject` data))
      (bind _returnvalue_2 (`SIOJsonObject.GetObjectArrayField` _returnvalue "objects"))
      (for _array_element _returnvalue_2
        ;[1 1 1] Extract position and spawn actor
        (bind _returnvalue_3 (`SIOJsonObject.GetNumberArrayField` _array_element "position"))
        (bind _returnvalue_4 (`|SpawnActorFromClass` "/Game/ZOurProject/Blueprint/SpaceObj.SpaceObj_C" (`KismetMathLibrary.Conv_VectorToTransform` (`KismetMathLibrary.MakeVector` (`|GetArrayItem` _returnvalue_3) (`|GetArrayItem` _returnvalue_3 1) (`|GetArrayItem` _returnvalue_3 2))) "Undefined" "OverrideRootScale" null null))
        ;[1 1 1] Set Name
        (set `/Game/ZOurProject/Blueprint/SpaceObj.name` (`SIOJsonObject.GetStringField` _array_element "name") _returnvalue_4)
        ;[1 1 1] setSpeed
        (bind _returnvalue_5 (`SIOJsonObject.GetNumberArrayField` _array_element "speed"))
        (set `/Game/ZOurProject/Blueprint/SpaceObj.speed` (`KismetMathLibrary.MakeVector` (`|GetArrayItem` _returnvalue_5) (`|GetArrayItem` _returnvalue_5 1) (`|GetArrayItem` _returnvalue_5 2)) _returnvalue_4)
        (`KismetArrayLibrary.Array_AddUnique` (`self.allObjects`) _returnvalue_4)))
    (:`newSimulation`
      (bind _returnvalue_6 (`SIOJsonValue.AsObject` data))
      (bind _returnvalue_7 (`SIOJsonObject.GetObjectArrayField` _returnvalue_6 "objects"))
      (for _array_element_2 _returnvalue_7
        (for _array_element_3 (`self.allObjects`)
          (bind _asspace_obj (cast `/Game/ZOurProject/Blueprint/SpaceObj` _array_element_3))
          (bind _returnvalue_8 (`SIOJsonObject.GetNumberArrayField` _array_element_2 "position"))
          (if (`KismetStringLibrary.EqualEqual_StrStr` (`SIOJsonObject.GetStringField` _array_element_2 "name") (`/Game/ZOurProject/Blueprint/SpaceObj.name` _asspace_obj))
            (`self.K2_SetActorTransform` _asspace_obj (`KismetMathLibrary.Conv_VectorToTransform` (`KismetMathLibrary.MakeVector` (`|GetArrayItem` _returnvalue_8) (`|GetArrayItem` _returnvalue_8 1) (`|GetArrayItem` _returnvalue_8 2))) false false)))))))

(fn `UserConstructionScript`)